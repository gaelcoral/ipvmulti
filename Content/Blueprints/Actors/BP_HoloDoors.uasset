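; BP_HoloDoors is a two-door actor that automatically toggles on a looping timer, with the doors offset vertically in opposite directions.
; ToggleDoors flips IsDoorAOpen on authority, and its OnRep function plays or reverses the DoorAnim timeline to follow the replicated state.
; The timeline's update lerps both doors inversely between DoorA's and DoorB's open positions, leaving closed positions unused.
; Overlap events are empty, and debug prints remain.
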(event OnComponentBeginOverlap(Box)
  (params (OverlappedComponent :type Primitive%20Component%20Object%20Reference) (OtherActor :type Actor%20Object%20Reference) (OtherComp :type Primitive%20Component%20Object%20Reference) (OtherBodyIndex :type Integer) (bFromSweep :type Boolean) (SweepResult :type Hit%20Result%20Structure%20%28by%20ref%29)))

(event OnComponentEndOverlap(Box)
  (params (OverlappedComponent :type Primitive%20Component%20Object%20Reference) (OtherActor :type Actor%20Object%20Reference) (OtherComp :type Primitive%20Component%20Object%20Reference) (OtherBodyIndex :type Integer)))

(event Collision|EventActorBeginOverlap
  (params (OtherActor :type Actor%20Object%20Reference)))

(event EventTick
  (params (DeltaSeconds :type Float%20%28single-precision%29)))

(event EventBeginPlay
  (Networking|SwitchHasAuthority
    (:Authority
      _)
    (:Remote
      _))
  (CallFunction|DoorAnimUpdateFunc)
  (Utilities|Time|SetTimerbyFunctionName 0 "ToggleDoors" 3.0 true)
  (bind _output_get (Variables|Default|SetDoorAClosedLocation (Variables|/Script/Engine.SceneComponent|GetRelativeLocation (Variables|Default|GetDoorA%20))))
  (bind _output_get_2 (Variables|Default|SetDoorAOpenLocation (+ _output_get (Math|Vector|MakeVector 0.0 0.0 2e+02))))
  (bind _output_get_3 (Variables|Default|SetDoorBClosedLocation (Variables|/Script/Engine.SceneComponent|GetRelativeLocation (Variables|Default|GetDoorB))))
  (bind _output_get_4 (Variables|Default|SetDoorBOpenLocation (+ _output_get_3 (Math|Vector|MakeVector 0.0 0.0 -2e+02))))
  (Development|PrintString (Utilities|String|ToString(Vector) _output_get_4)))

(fn ConstructionScript)

(fn ToggleDoors
  (Development|PrintString "jala ToggleDoors")
  (if (Ability|HasAuthority)
    (Variables|Default|SetbIsDoorAOpen (not (Variables|Default|GetbIsDoorAOpen)))))

(fn OnRepBIsDoorAOpen
  (Development|PrintString "jala OnRep ")
  (if (Variables|Default|GetbIsDoorAOpen)
    (Audio|Components|Audio|Play (Variables|Default|GetDoorAnim))
    (else
      (Utilities|String|Reverse (Variables|Default|GetDoorAnim)))))